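; BP_Robot_Orb is a playable orb robot that can interact with objects it overlaps.
; On possession it has the gameplay player controller set up the input mapping context, falling back to the test controller.
; When IA_Interact starts, it sends InteractMessage with itself to the first overlapping actor that implements BPI_Interact, so targets stay decoupled from the robot.
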(event Input|EnhancedActionEvents|EnhancedInputActionIA_Interact
  (params (ActionValue :type Boolean) (ElapsedSeconds :type Float%20%28double-precision%29) (TriggeredSeconds :type Float%20%28double-precision%29) (InputAction :type Input%20Action%20Object%20Reference :default "/Game/MechanicalRunaways/Inputs/Robot_Orb/IA_Actions/IA_Interact.IA_Interact"))
  (:Started
    (bind _array_element (Utilities|Array|ForEachLoopwithBreak (Collision|GetOverlappingActors 0 :!class /Script/Engine.Actor) :!label _label)
      (:LoopBody
        (if (Utilities|DoesObjectImplementInterface _array_element "/Game/MechanicalRunaways/Blueprints/Interfaces/BPI_Interact.BPI_Interact_C")
          (Class|BPIInteract|Interact(Message) _array_element self)
          (goto _label Break))))))

(event EventPossessed
  (params (NewController :type Controller%20Object%20Reference))
  (bind _asbp_gameplay_pc (Utilities|Casting|CastToBP_Gameplay_PC NewController)
    (:then
      (Default|SetUpInputMappingContext _asbp_gameplay_pc))
    (:CastFailed
      (bind _asbp_test_pc (Utilities|Casting|CastToBP_Test_PC NewController))
      (Default|SetupInputMappingContext _asbp_test_pc self))))

(fn ConstructionScript)