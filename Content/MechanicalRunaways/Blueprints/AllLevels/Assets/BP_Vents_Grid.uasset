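; BP_Vents_Grid is a powered vent grate that swings open and closed by rotating its mesh on pitch from its starting rotation.
; Power on and power off both set an owner, then call the multicast directly with authority or go through a server event without it.
; The multicast uses a FlipFlop to play or reverse a rotation-lerp timeline, so either power event toggles the grate rather than setting a specific state.
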(event Custom|Multicast_Open_Close_Door
  (Utilities|FlowControl|FlipFlop
    (:A
      (bind _alpha (Timeline|Timeline_Alpa_Loc Play)
        (:Update
          (Transformation|SetRelativeRotation (Variables|Default|GetVents_Grid) (Math|Rotator|Lerp(Rotator) (Variables|Default|GetStart_Vent_Rotation) (Variables|Default|GetEnd_Vent_Rotation) _alpha) false false))))
    (:B
      (Timeline|Timeline_Alpa_Loc Reverse))))

(event Custom|Server_Open_Close_Door
  (CallFunction|MulticastOpenCloseDoor))

(event EventBeginPlay
  (Variables|Default|SetStart_Vent_Rotation (Variables|/Script/Engine.SceneComponent|GetRelativeRotation (Variables|Default|GetVents_Grid)))
  (Variables|Default|SetEnd_Vent_Rotation (Math|Rotator|MakeRotator (.roll (Variables|Default|GetStart_Vent_Rotation)) (+ (.pitch (Variables|Default|GetStart_Vent_Rotation)) 1.2e+02) (.yaw (Variables|Default|GetStart_Vent_Rotation)))))

(event EventPowerOff
  (params (PlayerRef :type Controller%20Object%20Reference))
  (Actor|SetOwner 0)
  (if (Ability|HasAuthority (Components|GetOwner))
    (CallFunction|MulticastOpenCloseDoor)
    (else
      (CallFunction|ServerOpenCloseDoor))))

(event EventPoweron
  (params (PlayerRef :type Controller%20Object%20Reference))
  (Actor|SetOwner PlayerRef 0)
  (if (Ability|HasAuthority (Components|GetOwner))
    (CallFunction|MulticastOpenCloseDoor)
    (else
      (CallFunction|ServerOpenCloseDoor))))

(fn ConstructionScript)