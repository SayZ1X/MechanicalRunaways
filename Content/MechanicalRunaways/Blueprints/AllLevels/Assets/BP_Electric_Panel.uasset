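; BP_Electric_Panel is an interactable electric panel that toggles the filling state of a linked cable.
; Overlapping its collision shows a widget and makes the overlapping actor the panel's owner; leaving hides the widget and clears the owner.
; Interact goes to a multicast directly on authority or through a server event otherwise, where a FlipFlop sets the cable's IsFilling.
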(event OnComponentBeginOverlap(Interact_Collision)
  (params (OverlappedComponent :type Primitive%20Component%20Object%20Reference) (OtherActor :type Actor%20Object%20Reference) (OtherComp :type Primitive%20Component%20Object%20Reference) (OtherBodyIndex :type Integer) (bFromSweep :type Boolean) (SweepResult :type Hit%20Result%20Structure%20%28by%20ref%29))
  (if true
    (Rendering|SetVisibility (Variables|Default|GetWidget) true false)
    (Actor|SetOwner OtherActor)))

(event OnComponentEndOverlap(Interact_Collision)
  (params (OverlappedComponent :type Primitive%20Component%20Object%20Reference) (OtherActor :type Actor%20Object%20Reference) (OtherComp :type Primitive%20Component%20Object%20Reference) (OtherBodyIndex :type Integer))
  (if true
    (Rendering|SetVisibility (Variables|Default|GetWidget) false false)
    (Actor|SetOwner 0)))

(event Custom|Multicast_Activate_Electric_Panel
  (bind _linkedcable (Variables|Default|GetLinkedCable))
  (bind _isa (Utilities|FlowControl|FlipFlop)
    (:A
      _)
    (:B
      _))
  (Utilities|IsValid _linkedcable
    (:Is%20Valid
      (Variables|/Game/MechanicalRunaways/Blueprints/AllLevels/Assets/Power_Cable/BP_Power_Cable.BP_Power_Cable_C|SetisFilling? _linkedcable _isa))))

(event Custom|Server_Activate_Electric_Panel
  (CallFunction|MulticastActivateElectricPanel))

(event EventInteract
  (params (PlayerRef :type Controller%20Object%20Reference))
  (if (Ability|HasAuthority PlayerRef)
    (CallFunction|MulticastActivateElectricPanel)
    (else
      (CallFunction|ServerActivateElectricPanel))))

(fn ConstructionScript)