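; BP_Pressure_Plate_1 is a pressure plate triggered by actors tagged Robot_Orb, which drives a linked cable.
; When such an actor enters or leaves the Box trigger, it sets the LinkedCable's IsFilling flag on or off, provided a cable is linked.
; The same check plays or reverses a Timeline that linearly lowers and raises the plate's upper part.
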(event OnComponentBeginOverlap(Box)
  (params (OverlappedComponent :type Primitive%20Component%20Object%20Reference) (OtherActor :type Actor%20Object%20Reference) (OtherComp :type Primitive%20Component%20Object%20Reference) (OtherBodyIndex :type Integer) (bFromSweep :type Boolean) (SweepResult :type Hit%20Result%20Structure%20%28by%20ref%29))
  (bind _linked_cable (Variables|Default|GetLinked_Cable))
  (if (Actor|ActorHasTag OtherActor "Robot_Orb")
    (Utilities|IsValid _linked_cable
      (:Is%20Valid
        (Variables|/Game/MechanicalRunaways/Blueprints/AllLevels/Assets/Power_Cable/BP_Power_Cable.BP_Power_Cable_C|SetisFilling? _linked_cable true)
        (bind _alpha (Timeline|Timeline Play)
          (:Update
            (Transformation|SetRelativeLocation (Variables|Default|GetPressuer_Plate_Upper_Part) (Math|Interpolation|Ease :Function "Linear" :Alpha _alpha :B "0.000000,0.000000,-12.500000") false false)))))))

(event OnComponentEndOverlap(Box)
  (params (OverlappedComponent :type Primitive%20Component%20Object%20Reference) (OtherActor :type Actor%20Object%20Reference) (OtherComp :type Primitive%20Component%20Object%20Reference) (OtherBodyIndex :type Integer))
  (bind _linked_cable (Variables|Default|GetLinked_Cable))
  (if (Actor|ActorHasTag OtherActor "Robot_Orb")
    (Utilities|IsValid _linked_cable
      (:Is%20Valid
        (Variables|/Game/MechanicalRunaways/Blueprints/AllLevels/Assets/Power_Cable/BP_Power_Cable.BP_Power_Cable_C|SetisFilling? _linked_cable false)
        (bind _alpha (Timeline|Timeline Reverse)
          (:Update
            (Transformation|SetRelativeLocation (Variables|Default|GetPressuer_Plate_Upper_Part) (Math|Interpolation|Ease :Function "Linear" :Alpha _alpha :B "0.000000,0.000000,-12.500000") false false)))))))

(fn ConstructionScript)