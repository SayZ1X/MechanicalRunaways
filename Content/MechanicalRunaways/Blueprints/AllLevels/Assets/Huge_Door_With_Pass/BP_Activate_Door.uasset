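; BP_Activate_Door is an interactable that lets a player activate a linked object, likely a door.
; Its collision volume shows a prompt widget while an actor tagged Robot_Fly overlaps it and hides it on exit.
; Interact casts the player reference to BP_Test_PC and passes ActivateObject to ServerActivateObject, so activation is routed through the player rather than handled here.
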(event OnComponentBeginOverlap(Interact_Collision)
  (params (OverlappedComponent :type Primitive%20Component%20Object%20Reference) (OtherActor :type Actor%20Object%20Reference) (OtherComp :type Primitive%20Component%20Object%20Reference) (OtherBodyIndex :type Integer) (bFromSweep :type Boolean) (SweepResult :type Hit%20Result%20Structure%20%28by%20ref%29))
  (if (Actor|ActorHasTag OtherActor "Robot_Fly")
    (Rendering|SetVisibility (Variables|Default|GetWidget) true false)))

(event OnComponentEndOverlap(Interact_Collision)
  (params (OverlappedComponent :type Primitive%20Component%20Object%20Reference) (OtherActor :type Actor%20Object%20Reference) (OtherComp :type Primitive%20Component%20Object%20Reference) (OtherBodyIndex :type Integer))
  (if (Actor|ActorHasTag OtherActor "Robot_Fly")
    (Rendering|SetVisibility (Variables|Default|GetWidget) false false)))

(event EventInteract
  (params (PlayerRef :type Controller%20Object%20Reference))
  (bind _asbp_test_pc (Utilities|Casting|CastToBP_Test_PC PlayerRef))
  (Default|ServerActivateObject _asbp_test_pc (Variables|Default|GetActivateObject)))

(fn ConstructionScript)