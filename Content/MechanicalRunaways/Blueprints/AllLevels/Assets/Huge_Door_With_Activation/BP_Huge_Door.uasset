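; Two-part huge door that opens and closes vertically, and responds only after Activate_Door sets it active.
; Trigger volumes on each side toggle that side's prompt widget when an actor tagged Robot_Orb overlaps, though the second side's end-overlap checks the door's own tag.
; Interact routes through the player character's ServerOpenCloseDoor.
; Open_Close_Door flip-flops a timeline forward and back, lerping the halves apart from their starting heights.
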(event OnComponentBeginOverlap(Interact_Collision_First_Side)
  (params (OverlappedComponent :type Primitive%20Component%20Object%20Reference) (OtherActor :type Actor%20Object%20Reference) (OtherComp :type Primitive%20Component%20Object%20Reference) (OtherBodyIndex :type Integer) (bFromSweep :type Boolean) (SweepResult :type Hit%20Result%20Structure%20%28by%20ref%29))
  (if (Actor|ActorHasTag OtherActor "Robot_Orb")
    (if (Variables|Default|Getactivated?)
      (Rendering|SetVisibility (Variables|Default|GetWidget_First_Side) true false))))

(event OnComponentEndOverlap(Interact_Collision_First_Side)
  (params (OverlappedComponent :type Primitive%20Component%20Object%20Reference) (OtherActor :type Actor%20Object%20Reference) (OtherComp :type Primitive%20Component%20Object%20Reference) (OtherBodyIndex :type Integer))
  (if (Actor|ActorHasTag OtherActor "Robot_Orb")
    (if (Variables|Default|Getactivated?)
      (Rendering|SetVisibility (Variables|Default|GetWidget_First_Side) false false))))

(event OnComponentBeginOverlap(Interact_Collision_Second_Side)
  (params (OverlappedComponent :type Primitive%20Component%20Object%20Reference) (OtherActor :type Actor%20Object%20Reference) (OtherComp :type Primitive%20Component%20Object%20Reference) (OtherBodyIndex :type Integer) (bFromSweep :type Boolean) (SweepResult :type Hit%20Result%20Structure%20%28by%20ref%29))
  (if (Actor|ActorHasTag OtherActor "Robot_Orb")
    (if (Variables|Default|Getactivated?)
      (Rendering|SetVisibility (Variables|Default|GetWidget_Second_Side) true false))))

(event OnComponentEndOverlap(Interact_Collision_Second_Side)
  (params (OverlappedComponent :type Primitive%20Component%20Object%20Reference) (OtherActor :type Actor%20Object%20Reference) (OtherComp :type Primitive%20Component%20Object%20Reference) (OtherBodyIndex :type Integer))
  (if (Actor|ActorHasTag "Robot_Orb")
    (if (Variables|Default|Getactivated?)
      (Rendering|SetVisibility (Variables|Default|GetWidget_Second_Side) false false))))

(event Custom|Open_Close_Door
  (if (Variables|Default|Getactivated?)
    (Utilities|FlowControl|FlipFlop
      (:A
        (bind _bottom_part_loc (Timeline|Timeline_Alpa_Loc Play)
          (:Update
            (Transformation|SetRelativeLocation (Variables|Default|GetDoor_Bottom_Part) (Math|Vector|MakeVector 0.0 0.0 (Math|Float|Lerp (Variables|Default|GetStart_Bottom_Door_Part_Loc) (Variables|Default|GetEnd_Bottom_Door_Part_Loc) _bottom_part_loc)) false false)
            (Transformation|SetRelativeLocation (Variables|Default|GetDoor_Upper_Part) (Math|Vector|MakeVector 0.0 0.0 (Math|Float|Lerp (Variables|Default|GetStart_Upper_Door_Part_Loc) (Variables|Default|GetEnd_Upper_Door_Part_Loc) _bottom_part_loc)) false false))))
      (:B
        (Timeline|Timeline_Alpa_Loc Reverse)))))

(event Custom|Activate_Door
  (Variables|Default|Setactivated? true))

(event EventBeginPlay
  (bind _output_get (Variables|Default|SetStart_Bottom_Door_Part_Loc (.z (Variables|/Script/Engine.SceneComponent|GetRelativeLocation (Variables|Default|GetDoor_Bottom_Part)))))
  (Variables|Default|SetEnd_Bottom_Door_Part_Loc (- _output_get 3e+02))
  (bind _output_get_2 (Variables|Default|SetStart_Upper_Door_Part_Loc (.z (Variables|/Script/Engine.SceneComponent|GetRelativeLocation (Variables|Default|GetDoor_Upper_Part)))))
  (Variables|Default|SetEnd_Upper_Door_Part_Loc (- _output_get_2 -3.5e+02)))

(event EventInteract
  (params (PlayerRef :type Pawn%20Object%20Reference))
  (bind _asplayer_character (Utilities|Casting|CastToPlayer_Character PlayerRef))
  (Class|PlayerCharacter|ServerOpenCloseDoor _asplayer_character self))

(fn ConstructionScript)