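; BP_Door is a door that slides down and back up as a Player-tagged actor enters and leaves its Box trigger.
; BeginPlay stores the door's relative Z and an end position a fixed distance below it.
; Both overlap events call the same open routine, where a FlipFlop alternates between playing and reversing a timeline that lerps the height.
; The state therefore toggles per call rather than following whether the player is inside.
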(event OnComponentBeginOverlap(Box)
  (params (OverlappedComponent :type Primitive%20Component%20Object%20Reference) (OtherActor :type Actor%20Object%20Reference) (OtherComp :type Primitive%20Component%20Object%20Reference) (OtherBodyIndex :type Integer) (bFromSweep :type Boolean) (SweepResult :type Hit%20Result%20Structure%20%28by%20ref%29))
  (if (Actor|ActorHasTag OtherActor "Player")
    (CallFunction|OpenDoor)))

(event OnComponentEndOverlap(Box)
  (params (OverlappedComponent :type Primitive%20Component%20Object%20Reference) (OtherActor :type Actor%20Object%20Reference) (OtherComp :type Primitive%20Component%20Object%20Reference) (OtherBodyIndex :type Integer))
  (if (Actor|ActorHasTag OtherActor "Player")
    (CallFunction|OpenDoor)))

(event Custom|Open_Door
  (Utilities|FlowControl|FlipFlop
    (:A
      (bind _doorfloatalpha (Timeline|OpenDoorTimeLine Play)
        (:Update
          (Transformation|SetRelativeLocation (Variables|Default|GetDoor) (Math|Vector|MakeVector 0.0 0.0 (Math|Float|Lerp (Variables|Default|GetStartPos) (Variables|Default|GetEndPos) _doorfloatalpha)) false false))))
    (:B
      (Timeline|OpenDoorTimeLine Reverse))))

(event EventBeginPlay
  (bind _output_get (Variables|Default|SetStartPos (.z (Variables|/Script/Engine.SceneComponent|GetRelativeLocation (Variables|Default|GetDoor)))))
  (Variables|Default|SetEndPos (- _output_get 65.0)))

(fn ConstructionScript)