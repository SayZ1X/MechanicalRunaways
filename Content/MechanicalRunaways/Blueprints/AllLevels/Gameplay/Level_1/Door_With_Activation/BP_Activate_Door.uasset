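; BP_Activate_Door is a Level 1 interactable that activates a door through the player character.
; Its interaction collision shows or hides a widget when an actor tagged Robot_Fly enters or leaves it.
; The Interact event casts the caller to Player_Character and calls ServerActivateDoor with ActivateObject, handing the activation to the player's server-side call.
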(event OnComponentBeginOverlap(Interact_Collision)
  (params (OverlappedComponent :type Primitive%20Component%20Object%20Reference) (OtherActor :type Actor%20Object%20Reference) (OtherComp :type Primitive%20Component%20Object%20Reference) (OtherBodyIndex :type Integer) (bFromSweep :type Boolean) (SweepResult :type Hit%20Result%20Structure%20%28by%20ref%29))
  (if (Actor|ActorHasTag OtherActor "Robot_Fly")
    (Rendering|SetVisibility (Variables|Default|GetWidget) true false)))

(event OnComponentEndOverlap(Interact_Collision)
  (params (OverlappedComponent :type Primitive%20Component%20Object%20Reference) (OtherActor :type Actor%20Object%20Reference) (OtherComp :type Primitive%20Component%20Object%20Reference) (OtherBodyIndex :type Integer))
  (if (Actor|ActorHasTag OtherActor "Robot_Fly")
    (Rendering|SetVisibility (Variables|Default|GetWidget) false false)))

(event EventInteract
  (params (PlayerRef :type Pawn%20Object%20Reference))
  (bind _asplayer_character (Utilities|Casting|CastToPlayer_Character PlayerRef))
  (Class|PlayerCharacter|ServerActivateDoor _asplayer_character (Variables|Default|GetActivateObject)))

(fn ConstructionScript)